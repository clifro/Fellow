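; AIC_Enemy is the enemy AI controller, which runs the BT_Enemy behavior tree on BeginPlay.
; Perception updates feed the blackboard: a BP_Fellow_Hero becomes TargetActor only while alive and successfully sensed, otherwise the key is cleared.
; Every hero update also records the stimulus location as TargetLastPosition, including when sensing is lost.
; An update from any non-hero actor also clears TargetActor.
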(event OnTargetPerceptionUpdated(AIPerception)
  (params (Actor :type Actor%20Object%20Reference) (Stimulus :type AI%20Stimulus%20Structure))
  (bind (_age _expirationage _strength _stimuluslocation _receiverlocation _tag _bsuccessfullysensed) (Utilities|Struct|BreakAIStimulus Stimulus))
  (bind _asbp_fellow_hero (Utilities|Casting|CastToBP_Fellow_Hero Actor)
    (:then
      (AI|Components|Blackboard|SetValueasObject (Variables|Default|GetBlackboard) (Utilities|Name|MakeLiteralName "TargetActor") (Utilities|SelectObject Actor 0 (and (Class|PFCharacter|IsAlive _asbp_fellow_hero) _bsuccessfullysensed)))
      (AI|Components|Blackboard|SetValueasVector (Variables|Default|GetBlackboard) (Utilities|Name|MakeLiteralName "TargetLastPosition") _stimuluslocation))
    (:CastFailed
      (AI|Components|Blackboard|SetValueasObject (Variables|Default|GetBlackboard) (Utilities|Name|MakeLiteralName "TargetActor") 0))))

(event EventBeginPlay
  (AI|RunBehaviorTree "/Game/Blueprints/AI/BT_Enemy.BT_Enemy"))

(event EventTick
  (params (DeltaSeconds :type Float%20%28single-precision%29)))

(fn ConstructionScript)