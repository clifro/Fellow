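; Enemy character Blueprint that overrides how an AI enemy aims at a hero target.
; Aim starts at the weapon socket, and the target comes from the blackboard's TargetActor.
; For a hero target, it line-traces toward several aim sockets on the hero's mesh and randomly picks among directions that hit a physics body.
; It falls back to parent aiming when the socket, target or candidate directions are missing.
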(event Collision|EventActorBeginOverlap
  (params (OtherActor :type Actor%20Object%20Reference)))

(event EventTick
  (params (DeltaSeconds :type Float%20%28single-precision%29)))

(fn ConstructionScript
  (|CallParentFunction))

(fn GetAimDirection
  (bind _returnvalue (AI|GetBlackboard 0))
  (bind _returnvalue_2 (Utilities|Name|MakeLiteralName "TargetActor"))
  (bind _returnvalue_3 (AI|Components|Blackboard|GetValueasObject _returnvalue _returnvalue_2))
  (Utilities|IsValid _returnvalue
    (:Is%20Valid
      (Utilities|IsValid _returnvalue_3
        (:Is%20Valid
          (bind _asbp_fellow_hero (Utilities|Casting|CastToBP_Fellow_Hero _returnvalue_3)
            (:then
              (bind _returnvalue_4 (CallFunction|GetAimRandomDirection (Variables|/Script/Engine.Character|GetMesh _asbp_fellow_hero)))
              (return _returnvalue_4))
            (:CastFailed
              _)))
        (:Is%20Not%20Valid
          _)))
    (:Is%20Not%20Valid
      _))
  (return (|CallParentFunction)))

(fn GetAimStartLocation
  (bind _mesh (Variables|Character|GetMesh))
  (if (Transformation|DoesSocketExist _mesh "Socket_Weapon")
    (return (Transformation|GetSocketLocation _mesh "Socket_Weapon"))
    (else
      (return (|CallParentFunction)))))

(fn GetAimRandomDirection
  (params (Mesh :type Mesh%20Component%20Object%20Reference))
  (bind _returnvalue (CallFunction|GetAimStartLocation))
  (bind _aimdirections (LocalVariables|GetAimDirections))
  (for _array_element (Utilities|Array|MakeArray (Utilities|Name|MakeLiteralName "Socket_Aim1") (Utilities|Name|MakeLiteralName "Socket_Aim2") (Utilities|Name|MakeLiteralName "Socket_Aim3") (Utilities|Name|MakeLiteralName "Socket_Aim4H"))
    (if (Transformation|DoesSocketExist Mesh _array_element)
      (bind _outhit (Collision|LineTraceForObjects _returnvalue (+ _returnvalue (* (Math|Vector|GetUnitDirection(Vector) _returnvalue (Transformation|GetSocketLocation Mesh _array_element)) 2e+03)) (Utilities|Array|MakeArray "ObjectTypeQuery4") false (Utilities|Array|MakeArray self) "None"))
      (if (.bBlockingHit (Collision|BreakHitResult _outhit))
        (Utilities|Array|AddUnique (LocalVariables|GetAimDirections) (Math|Vector|GetUnitDirection(Vector) _returnvalue (Transformation|GetSocketLocation Mesh _array_element))))))
  (if (> (Utilities|Array|Length _aimdirections) 0)
    (return (.OutItem (Utilities|Array|Random _aimdirections)))
    (else
      (return (|CallParentFunction)))))