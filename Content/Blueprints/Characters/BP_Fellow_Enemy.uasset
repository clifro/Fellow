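; BP_Fellow_Enemy is an enemy character Blueprint that overrides where its aim starts and which direction it points.
; Aim starts at the mesh's weapon socket, falling back to the parent implementation.
; GetAimDirection reads TargetActor from the blackboard and picks a random direction toward the target hero's aim sockets, otherwise using the parent's direction.
; Each socket gets a line trace, but its result is unused, so obstructions do not filter candidates.
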(event Collision|EventActorBeginOverlap
  (params (OtherActor :type Actor%20Object%20Reference)))

(event EventTick
  (params (DeltaSeconds :type Float%20%28single-precision%29)))

(fn ConstructionScript
  (|CallParentFunction))

(fn GetAimDirection
  (bind _returnvalue (AI|GetBlackboard 0))
  (bind _returnvalue_2 (CallFunction|GetAimStartLocation))
  (bind _returnvalue_3 (Utilities|Name|MakeLiteralName "TargetActor"))
  (bind _aimpositions (Variables|Default|GetAimPositions))
  (bind _returnvalue_4 (AI|Components|Blackboard|GetValueasObject _returnvalue _returnvalue_3))
  (Utilities|Array|Clear (Variables|Default|GetAimPositions))
  (Utilities|IsValid _returnvalue
    (:Is%20Valid
      (Utilities|IsValid _returnvalue_4
        (:Is%20Valid
          (bind _asbp_fellow_hero (Utilities|Casting|CastToBP_Fellow_Hero _returnvalue_4)
            (:then
              (for _array_element (Utilities|Array|MakeArray (Utilities|Name|MakeLiteralName "Socket_Aim1") (Utilities|Name|MakeLiteralName "Socket_Aim2") (Utilities|Name|MakeLiteralName "Socket_Aim3") (Utilities|Name|MakeLiteralName "Socket_Aim4H"))
                (if (Transformation|DoesSocketExist (Variables|/Script/Engine.Character|GetMesh _asbp_fellow_hero) _array_element)
                  (bind _outhit (Collision|LineTraceForObjects _returnvalue_2 (+ _returnvalue_2 (* (Math|Vector|GetUnitDirection(Vector) _returnvalue_2 (Transformation|GetSocketLocation (Variables|/Script/Engine.Character|GetMesh _asbp_fellow_hero) _array_element)) 2e+03)) (Utilities|Array|MakeArray "ObjectTypeQuery4") false (Utilities|Array|MakeArray self) "None"))
                  (Utilities|Array|AddUnique (Variables|Default|GetAimPositions) (Math|Vector|GetUnitDirection(Vector) _returnvalue_2 (Transformation|GetSocketLocation (Variables|/Script/Engine.Character|GetMesh _asbp_fellow_hero) _array_element)))))
              (if (> (Utilities|Array|Length _aimpositions) 0)
                (return (.OutItem (Utilities|Array|Random _aimpositions)))
                (else
                  _)))
            (:CastFailed
              _)))
        (:Is%20Not%20Valid
          _)))
    (:Is%20Not%20Valid
      _))
  (return (|CallParentFunction)))

(fn GetAimStartLocation
  (bind _mesh (Variables|Character|GetMesh))
  (if (Transformation|DoesSocketExist _mesh "Socket_Weapon")
    (return (Transformation|GetSocketLocation _mesh "Socket_Weapon"))
    (else
      (return (|CallParentFunction)))))